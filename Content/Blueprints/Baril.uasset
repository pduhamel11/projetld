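; Baril is a destructible barrel Blueprint that explodes after taking enough FirstPersonProjectile hits.
; Each projectile hit on its static mesh lowers BarilWhiteHealth by a fixed amount, then tests for exactly zero.
; At zero it spawns TriggerSphereBaril_Blueprint, prints a debug string, plays explosion particles and sound, then destroys itself.
; The trigger's spawn transform reads from a self-type cast that never executes, unlike the effects, which use the actor's own location.
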(event OnComponentHit(StaticMeshComponent)
  (params (OtherActor :type Actor%20Object%20Reference) (OtherComp :type Primitive%20Component%20Object%20Reference) (NormalImpulse :type Vector :default "0, 0, 0") (Hit :type Hit%20Result%20Structure%20%28by%20ref%29))
  (Utilities|Casting|CastToFirstPersonProjectile OtherActor)
  (Variables|Default|SetBarilWhiteHealth (- (Variables|Default|GetBarilWhiteHealth) 0.5))
  (if (== (Variables|Default|GetBarilWhiteHealth) 0.0)
    (Game|SpawnActorfromClass "/Game/TriggerSphereBaril_Blueprint.TriggerSphereBaril_Blueprint_C" (Transformation|GetActorTransform (stale _asbaril)) "Undefined" 0 0)
    (Development|PrintString "Hello")
    (Effects|SpawnEmitteratLocation "/Game/StarterContent/Particles/P_Explosion.P_Explosion" (Transformation|GetActorLocation))
    (Audio|PlaySoundatLocation "/Game/StarterContent/Audio/Explosion01.Explosion01" (Transformation|GetActorLocation))
    (Actor|DestroyActor)))

(event EventBeginPlay)

(event EventActorBeginOverlap
  (params (OtherActor :type Actor%20Object%20Reference)))

(event EventTick
  (params (DeltaSeconds :type Float%20%28single-precision%29)))

(fn ConstructionScript)